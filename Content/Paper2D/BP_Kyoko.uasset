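; BP_Kyoko is a Paper2D flipbook character that always turns to face the player camera.
; It looks up animations by name in a FlipBooks map, applies them to its sprite and returns their duration.
; On BeginPlay it plays a start animation, and on damage a hit animation, each returning to idle after a retriggerable delay of that length.
; Every tick it sets only its yaw toward the camera, billboard-style.
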(event EventBeginPlay
  (bind _returnvalue (CallFunction|SetFlipBook "Start"))
  (Utilities|FlowControl|RetriggerableDelay _returnvalue)
  (CallFunction|SetFlipBook "Idle"))

(event EventTick
  (params (DeltaSeconds :type Float%20%28single-precision%29))
  (Transformation|SetActorRotation (Math|Rotator|MakeRotator 0.0 0.0 (- (.yaw (Math|Rotator|FindLookatRotation (Transformation|GetActorLocation) (Camera|GetCameraLocation (Game|GetPlayerCameraManager 0)))) 9e+01))))

(event Game|Damage|EventAnyDamage
  (params (Damage :type Float%20%28single-precision%29) (DamageType :type Damage%20Type%20Object%20Reference) (InstigatedBy :type Controller%20Object%20Reference) (DamageCauser :type Actor%20Object%20Reference))
  (bind _returnvalue (CallFunction|SetFlipBook "Hitted"))
  (Utilities|FlowControl|RetriggerableDelay _returnvalue)
  (CallFunction|SetFlipBook "Idle"))

(fn ConstructionScript)

(fn SetFlipBook
  (params (Name :type Name))
  (bind _flipbooks (Variables|Default|GetFlipBooks))
  (bind _value (Utilities|Map|Find _flipbooks Name))
  (Sprite|SetFlipbook (Variables|Default|GetSprite) _value)
  (return (Class|PaperFlipbook|GetTotalDuration _value)))