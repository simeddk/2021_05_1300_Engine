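; Replication test chest, named for owner-only relevancy, that displays the username of the player overlapping it.
; Box overlap makes the other actor the owner; on authority, a BP_CPlayer triggers a client event that reads the name from its UserNameWidget.
; That event passes the name to a server event, which sets the RepNotify Text variable, and OnRep_Text updates the TextRender.
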(event OnComponentBeginOverlap(Box)
  (params (OverlappedComponent :type Primitive%20Component%20Object%20Reference) (OtherActor :type Actor%20Object%20Reference) (OtherComp :type Primitive%20Component%20Object%20Reference) (OtherBodyIndex :type Integer) (bFromSweep :type Boolean) (SweepResult :type Hit%20Result%20Structure%20%28by%20ref%29))
  (Actor|SetOwner OtherActor)
  (Networking|SwitchHasAuthority
    (:Authority
      (bind _asbp_cplayer (Utilities|Casting|CastToBP_CPlayer OtherActor))
      (CallFunction|ClientGetTextfromWidget _asbp_cplayer))))

(event Custom|Client_GetTextFromWidget
  (params (InPlayer :type BP%20C%20Player%20Object%20Reference))
  (CallFunction|ServerSetText (Class|TextBlock|GetText (Variables|/Game/Widgets/WB_UserName.WB_UserName_C|GetUser (Variables|/Game/Player/BP_CPlayer.BP_CPlayer_C|GetUserNameWidget InPlayer)))))

(event Custom|Server_SetText
  (params (Text :type Text))
  (Variables|Default|SetText Text))

(fn ConstructionScript
  (|CallParentFunction))

(fn OnRepText
  (Rendering|Components|TextRender|SetText (Variables|Default|GetTextRender) (Variables|Default|GetText)))