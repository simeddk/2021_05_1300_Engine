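; BP_Chest is a toggleable chest that demonstrates replication approaches, selected by ReplicationType: none, multicast, RepNotify or both.
; The non-replicated and multicast paths animate the lid with a flip-flopped Timeline and switch emissive intensity on finish, with multicast adding sound and particles.
; RepNotify flips Open, whose OnRep snaps the lid; Both chains this after the multicast animation.
; Construction creates the dynamic material and sizes an optional net cull distance sphere.
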(event Custom|Toggle
  (switch Utilities|FlowControl|Switch|SwitchonEReplicationType (Variables|Default|GetReplicationType)
    (:NewEnumerator0
      (CallFunction|ToggleNoReplication))
    (:NewEnumerator1
      (CallFunction|ToggleMulticast))
    (:NewEnumerator2
      (CallFunction|ToggleRepNotify))
    (:NewEnumerator3
      (CallFunction|ToggleMulticast))))

(event Custom|Toggle_RepNotify
  (Variables|Default|SetOpen (not (Variables|Default|GetOpen))))

(event Custom|Toggle_NoReplication
  (bind _isa (Utilities|FlowControl|FlipFlop)
    (:A
      (bind _alpha (Timeline|Timeline PlayFromStart)
        (:Update
          (CallFunction|ToggleTop _alpha))
        (:Finished
          (CallFunction|ToggleEmissive _isa)
          (if (Utilities|Enum|Equal(Enum) (Variables|Default|GetReplicationType) "NewEnumerator3")
            (CallFunction|ToggleRepNotify)))))
    (:B
      (Timeline|Timeline ReverseFromEnd))))

(event Custom|Toggle_Multicast
  (|PlayEffect)
  (bind _isa (Utilities|FlowControl|FlipFlop)
    (:A
      (bind _alpha (Timeline|Timeline PlayFromStart)
        (:Update
          (CallFunction|ToggleTop _alpha))
        (:Finished
          (CallFunction|ToggleEmissive _isa)
          (if (Utilities|Enum|Equal(Enum) (Variables|Default|GetReplicationType) "NewEnumerator3")
            (CallFunction|ToggleRepNotify)))))
    (:B
      (Timeline|Timeline ReverseFromEnd))))

(fn ConstructionScript
  (CallFunction|SetMaterial)
  (Transformation|SetWorldScale3D (Variables|Default|GetSphere) (Math|Conversions|ToVector(Float) (* (Math|Float|Sqrt (Variables|Default|GetNetCullDistanceSquared)) 2.0)))
  (Rendering|SetVisibility (Variables|Default|GetSphere) (Variables|Default|GetVisibleNetCullDistance) false))

(fn SetMaterial
  (bind _returnvalue (Rendering|Material|CreateDynamicMaterialInstance "/Game/Materials/Mi_Chest.Mi_Chest" "None" :!class /Script/Engine.KismetMaterialLibrary))
  (bind _output_get (Variables|Default|SetMaterial _returnvalue))
  (Rendering|Material|SetMaterial (Variables|Default|GetTop) 0 _output_get)
  (Rendering|Material|SetVectorParameterValue _output_get "Emissive" (Variables|Default|GetEmissive) :!class /Script/Engine.MaterialInstanceDynamic)
  (Rendering|Material|SetScalarParameterValue _output_get "Intensity" (Variables|Default|GetIntensity) :!class /Script/Engine.MaterialInstanceDynamic))

(fn ToggleTop
  (params (Alpha :type Float%20%28single-precision%29))
  (Transformation|SetRelativeRotation (Variables|Default|GetTop) (Math|Rotator|Lerp(Rotator) "0, 0, 0" "120.000000, 0,0.000000" Alpha) false false))

(fn ToggleEmissive
  (params (bPickA :type Boolean))
  (Rendering|Material|SetScalarParameterValue (Variables|Default|GetMaterial) "Intensity" (Math|Float|SelectFloat 0.0 (Variables|Default|GetIntensity) bPickA) :!class /Script/Engine.MaterialInstanceDynamic))

(fn OnRepOpen
  (Transformation|SetRelativeRotation (Variables|Default|GetTop) (Math|Rotator|SelectRotator "130.000000,0.000000, 0" "0.000000, 0,0.000000" (Variables|Default|GetOpen)) false false))