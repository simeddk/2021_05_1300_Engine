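; BP_Variable_OnlyAuthority is a replication example actor that shows a changing text value set only by the authority.
; On BeginPlay, the authority starts a looping one-second timer that assigns Display a random pick from the first three Contents entries and updates the TextRender.
; Display uses a RepNotify, whose OnRep_Display function applies the replicated value to the TextRender.
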(event Custom|UpdateperSecond
  (bind _output_get (Variables|Default|SetDisplay (Utilities|Array|Get(acopy) (Variables|Default|GetContents) (Math|Random|RandomIntegerinRange 0 2))))
  (Rendering|Components|TextRender|SetText (Variables|Default|GetTextRender) _output_get))

(event EventBeginPlay
  (|CallParentFunction)
  (Networking|SwitchHasAuthority
    (:Authority
      (Utilities|Time|SetTimerbyEvent (delegate Custom|UpdateperSecond) 1.0 true))))

(fn ConstructionScript
  (|CallParentFunction))

(fn OnRepDisplay
  (Rendering|Components|TextRender|SetText (Variables|Default|GetTextRender) (Variables|Default|GetDisplay)))