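; Test chest for owner-based replication that shows the name of the player who overlaps its box.
; On overlap it sets that actor as owner, then on authority sends BP_CPlayer to a client event that reads the name from the player's UserNameWidget.
; That name returns through a server event into Text, whose OnRep updates the TextRender.
; Taking ownership gives the client-to-server round trip an owning connection.
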(event OnComponentBeginOverlap(Box)
  (params (OverlappedComponent :type Primitive%20Component%20Object%20Reference) (OtherActor :type Actor%20Object%20Reference) (OtherComp :type Primitive%20Component%20Object%20Reference) (OtherBodyIndex :type Integer) (bFromSweep :type Boolean) (SweepResult :type Hit%20Result%20Structure%20%28by%20ref%29))
  (Actor|SetOwner OtherActor)
  (Networking|SwitchHasAuthority
    (:Authority
      (bind _asbp_cplayer (Utilities|Casting|CastToBP_CPlayer OtherActor))
      (CallFunction|ClinetGetTextfromWidget _asbp_cplayer))))

(event Custom|Clinet_GetTextFromWidget
  (params (Player :type BP%20C%20Player%20Object%20Reference))
  (CallFunction|ServerSetText (Class|TextBlock|GetText (Variables|/Game/Widgets/WB_UserName.WB_UserName_C|GetUser (Variables|/Game/Player/BP_CPlayer.BP_CPlayer_C|GetUserNameWidget Player)))))

(event Custom|Server_SetText
  (params (InText :type Text))
  (Variables|Default|SetText InText))

(fn ConstructionScript
  (|CallParentFunction))

(fn OnRepText
  (Rendering|Components|TextRender|SetText (Variables|Default|GetTextRender) (Variables|Default|GetText)))