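; BP_Chest_NetCull is a chest actor in the replication objects folder, named for net culling, that flags players standing in its overlap area.
; Begin and end overlap cast the other actor to BP_CPlayer, set its Overlapped flag true or false, and print its name.
; A RepNotify on the Text variable updates the TextRender, though no graph here writes that variable.
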(event Collision|EventActorBeginOverlap
  (params (OtherActor :type Actor%20Object%20Reference))
  (bind _asbp_cplayer (Utilities|Casting|CastToBP_CPlayer OtherActor))
  (Variables|/Game/Player/BP_CPlayer.BP_CPlayer_C|SetOverlapped _asbp_cplayer true)
  (Development|PrintString (Utilities|GetDisplayName _asbp_cplayer)))

(event Collision|EventActorEndOverlap
  (params (OtherActor :type Actor%20Object%20Reference))
  (bind _asbp_cplayer (Utilities|Casting|CastToBP_CPlayer OtherActor))
  (Variables|/Game/Player/BP_CPlayer.BP_CPlayer_C|SetOverlapped _asbp_cplayer false)
  (Development|PrintString (Utilities|GetDisplayName _asbp_cplayer)))

(fn ConstructionScript
  (|CallParentFunction))

(fn OnRepText
  (Rendering|Components|TextRender|SetText (Variables|Default|GetTextRender) (Variables|Default|GetText)))