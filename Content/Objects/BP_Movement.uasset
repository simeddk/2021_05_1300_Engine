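; Test-style moving actor that oscillates 200 units along its up vector and sizes its static mesh from its net cull distance.
; On authority only, a half-speed timeline lerps the location between start and end, with a FlipFlop on Finished alternating forward and reverse playback endlessly.
; The construction script scales the mesh to twice the square root of NetCullDistanceSquared, apparently to visualize the relevancy range.
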(event EventBeginPlay
  (bind _returnvalue (Transformation|GetActorLocation))
  (|CallParentFunction)
  (Networking|SwitchHasAuthority
    (:Authority
      (Variables|Default|SetStart _returnvalue)
      (Variables|Default|SetEnd (+ _returnvalue (* (Transformation|GetActorUpVector) 2e+02)))
      (Components|Timeline|SetPlayRate (Variables|Default|GetTime) 0.5)
      (Utilities|FlowControl|FlipFlop :!label _label
        (:A
          (bind _alpha (Timeline|Time PlayFromStart)
            (:Update
              (Transformation|SetActorLocation (Math|Vector|Lerp(Vector) (Variables|Default|GetStart) (Variables|Default|GetEnd) _alpha) false false))
            (:Finished
              (goto _label))))
        (:B
          (Timeline|Time ReverseFromEnd))))))

(fn ConstructionScript
  (|CallParentFunction)
  (Transformation|SetWorldScale3D (Variables|Default|GetStaticMesh) (Math|Conversions|ToVector(Float) (* (Math|Float|Sqrt (Variables|Default|GetNetCullDistanceSquared)) 2.0))))